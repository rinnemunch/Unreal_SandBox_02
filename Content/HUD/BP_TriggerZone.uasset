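; BP_TriggerZone is a trigger actor that shows a WBP_HUDTip widget when the player walks into its box.
; BeginPlay caches the player's BP_ThirdPersonCharacter, and the box's begin-overlap reacts only to that actor.
; A DoOnce limits it to the first entry, creating the widget and adding it to the viewport.
; A Delay follows with nothing after it, so this Blueprint never removes the tip.
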(event OnComponentBeginOverlap(Box)
  (params (OverlappedComponent :type Primitive%20Component%20Object%20Reference) (OtherActor :type Actor%20Object%20Reference) (OtherComp :type Primitive%20Component%20Object%20Reference) (OtherBodyIndex :type Integer) (bFromSweep :type Boolean) (SweepResult :type Hit%20Result%20Structure%20%28by%20ref%29))
  (if (== OtherActor (Variables|Default|GetAs%20BP%20Third%20Person%20Character))
    (Utilities|FlowControl|DoOnce false
      (:Completed
        (bind _returnvalue (UserInterface|CreateWidget "/Game/HUD/WBP_HUDTip.WBP_HUDTip_C" (Game|GetPlayerController 0)))
        (bind _output_get (Variables|Default|SetHUDRef _returnvalue))
        (UserInterface|Viewport|AddtoViewport _output_get 0)
        (Utilities|FlowControl|Delay 4.5)))))

(event EventBeginPlay
  (bind _asbp_third_person_character (Utilities|Casting|CastToBP_ThirdPersonCharacter (Game|GetPlayerCharacter 0)))
  (Variables|Default|SetAs%20BP%20Third%20Person%20Character _asbp_third_person_character))

(event Collision|EventActorBeginOverlap
  (params (OtherActor :type Actor%20Object%20Reference)))

(event EventTick
  (params (DeltaSeconds :type Float%20%28single-precision%29)))

(fn ConstructionScript)